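; BP_hero is the player hero that constantly moves forward along world X, with input steering it sideways along Y.
; Each tick it also applies a swept downward offset along the Box's inverted up vector, scaled by FallSpeed, as custom falling.
; Jump input resets GroundLevel and plays a Timeline, but the jump is unfinished: it sets the Box to world origin, leaving the height and Lerp nodes unwired.
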(event `EnhancedInput|/Game/Shifter/input/IA_jump`
  (params (ActionValue :type Boolean) (ElapsedSeconds :type "Float (double-precision)") (TriggeredSeconds :type "Float (double-precision)") (InputAction :type "InputAction Object Reference" :default "/Game/Shifter/input/IA_jump.IA_jump"))
  (:`Triggered`
    (set `self.GroundLevel` 0.0)
    (`Timeline|Шкала времени` :!via `PlayFromStart` ; Add Timeline
      (:`Update`
        (`SceneComponent.K2_SetWorldLocation` (`self.Box`) (0.0 0.0 0.0) false false)))))

(event `EnhancedInput|/Game/Shifter/input/IA_rightleft`
  (params (ActionValue :type "Float (double-precision)") (ElapsedSeconds :type "Float (double-precision)") (TriggeredSeconds :type "Float (double-precision)") (InputAction :type "InputAction Object Reference" :default "/Game/Shifter/input/IA_rightleft.IA_rightleft"))
  (:`Triggered`
    (`self.AddMovementInput` (0.0 1.0 0.0) ActionValue)))

(event `self.ReceiveTick`
  (params (DeltaSeconds :type "Float (single-precision)"))
  (`|ExecutionSequence`
    (:`then_0`
      (`self.AddMovementInput` (1.0 0.0 0.0)))
    (:`then_1`
      (`self.K2_AddActorWorldOffset` (* (* DeltaSeconds (`self.FallSpeed`)) (`KismetMathLibrary.NegateVector` (`SceneComponent.GetUpVector` (`self.Box`)))) true) ; нода для смещения
    )))

(fn `UserConstructionScript`)