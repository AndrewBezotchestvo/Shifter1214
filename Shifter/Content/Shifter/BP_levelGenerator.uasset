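; BP_levelGenerator endlessly spawns rows of BP_cube ahead of the player along X, forming a three-wide track.
; Tick calls GenerateRow whenever the last row is within range of the player, stepping cubes along Y before advancing X.
; RotateCube turns the two outer cubes in opposite directions and gives them random meshes from Variants.
; Tick also destroys the oldest cube, one per frame, while the count exceeds its cap.
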(event `GenerateRow`
  (bind (_lastblockposition_x _lastblockposition_y _lastblockposition_z) (`KismetMathLibrary.BreakVector` (`self.LastBlockPosition`)))
  (bind _lastblockposition_x_2 (`KismetMathLibrary.BreakVector` (`self.LastBlockPosition`)))
  (for _index (range 3)
    (bind _returnvalue (`|SpawnActorFromClass` "/Game/Shifter/BP_cube.BP_cube_C" (`KismetMathLibrary.MakeTransform` (`KismetMathLibrary.MakeVector` _lastblockposition_x (+ (`self.BlockOffset`) _lastblockposition_y) _lastblockposition_z)) "Undefined" "MultiplyWithRoot" null null))
    (`self.RotateCube` _index _returnvalue)
    (set `self.LastBlockPosition` (`self.K2_GetActorLocation` _returnvalue))
    (`KismetArrayLibrary.Array_Add` (`self.Cubes`) _returnvalue))
  (set `self.LastBlockPosition` (`KismetMathLibrary.MakeVector` (+ (`self.BlockOffset`) _lastblockposition_x_2))))

(event `self.ReceiveBeginPlay`)

(event `self.ReceiveTick`
  (params (DeltaSeconds :type "Float (single-precision)"))
  (bind _lastblockposition_x (`KismetMathLibrary.BreakVector` (`self.LastBlockPosition`)))
  (bind _cubes (`self.Cubes`))
  (`|ExecutionSequence`
    (:`then_0`
      (bind _output_get (set `self.PlayerPosition` (`self.K2_GetActorLocation` (`GameplayStatics.GetPlayerPawn` 0))))
      (if (> 1500.0 (- _lastblockposition_x (.x _output_get)))
        (`self.GenerateRow`)))
    (:`then_1`
      (if (> (`KismetArrayLibrary.Array_Length` (`self.Cubes`)) 100)
        (`self.K2_DestroyActor` (`|GetArrayItem` _cubes))
        (`KismetArrayLibrary.Array_Remove` _cubes)))))

(event `RotateCube`
  (params (Selection :type Integer) (`Цель` :type "/Game/Shifter/BP_cube Object Reference"))
  (switch `int` Selection
    (:`0`
      (`SceneComponent.K2_SetWorldRotation` (`Actor.RootComponent` `Цель`) (struct :`Yaw` -90.0) false false))
    (:`2`
      (`SceneComponent.K2_SetWorldRotation` (`Actor.RootComponent` `Цель`) (struct :`Yaw` 90.0) false false)))
  (`StaticMeshComponent.SetStaticMesh` (`/Game/Shifter/BP_cube.StaticMesh` `Цель`) (`KismetArrayLibrary.Array_Random` (`self.Variants`))))

(fn `UserConstructionScript`)